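; BallCharacter is a player-controlled character Blueprint that handles basic planar movement input.
; The MoveForward and MoveSide axis events add movement input only while Health is above zero.
; Directions come from the forward and right vectors of a zero rotation, so movement follows fixed world axes regardless of character or camera facing.
; BeginPlay, Tick, overlap and the construction script are empty.
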(event EventBeginPlay)

(event Collision|EventActorBeginOverlap
  (params (OtherActor :type Actor%20Object%20Reference)))

(event EventTick
  (params (DeltaSeconds :type Float%20%28single-precision%29)))

(event Input|AxisEvents|InputAxisMoveForward
  (params (AxisValue :type Float%20%28single-precision%29))
  (if (> (Variables|Default|GetHealth) 0.0)
    (Pawn|Input|AddMovementInput (Math|Vector|GetForwardVector "0, 0, 0") AxisValue false)))

(event Input|AxisEvents|InputAxisMoveSide
  (params (AxisValue :type Float%20%28single-precision%29))
  (if (> (Variables|Default|GetHealth) 0.0)
    (Pawn|Input|AddMovementInput (Math|Vector|GetRightVector "0, 0, 0") AxisValue false)))

(fn ConstructionScript)