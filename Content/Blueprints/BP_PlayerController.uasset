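; BP_PlayerController is a player controller that owns the player's HUD, showing health and the end-of-game message.
; On BeginPlay it creates the BP_HUD widget, stores the reference and adds it to the viewport.
; UpdateHealth sets the health bar from a 0–100 value, then writes a win or caught message based on the IsGameWon and IsGameLost flags, with winning checked first.
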(event Custom|CreateHUD
  (bind _returnvalue (UserInterface|CreateWidget "/Game/UI/HUD/BP_HUD.BP_HUD_C"))
  (bind _output_get (Variables|Default|SetHUDRef _returnvalue))
  (UserInterface|Viewport|AddtoViewport _output_get 0))

(event Custom|UpdateHealth
  (params (NewHealth :type Float%20%28double-precision%29))
  (Progress|SetPercent (Variables|/Game/UI/HUD/BP_HUD.BP_HUD_C|GetHealthBar (Variables|Default|GetHUDRef)) (/ NewHealth 1e+02))
  (if (Variables|Default|GetIsGameWon)
    (Rendering|Components|TextRender|SetText (Variables|/Game/UI/HUD/BP_HUD.BP_HUD_C|GetGameEndText (Variables|Default|GetHUDRef)) "You won it!")
    (elif (Variables|Default|GetIsGameLost)
      (Rendering|Components|TextRender|SetText (Variables|/Game/UI/HUD/BP_HUD.BP_HUD_C|GetGameEndText (Variables|Default|GetHUDRef)) "You've been caught"))))

(event EventBeginPlay
  (CallFunction|CreateHUD))

(event EventTick
  (params (DeltaSeconds :type Float%20%28single-precision%29)))

(fn ConstructionScript)