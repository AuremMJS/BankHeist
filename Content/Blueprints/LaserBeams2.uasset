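; Laser beam hazard that drains the BallCharacter's health while the ball crosses the line between its two nodes.
; BeginPlay passes both nodes and the heights of their position markers to SetLaserNodeParams.
; Each Tick, a Camera-channel trace between the nodes, drawn as a debug line, applies fixed per-frame damage on a hit.
; It then updates health through BP_PlayerController and flags the game as lost at zero.
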(event EventBeginPlay
  (Class|LaserBeamBase|SetLaserNodeParams (Variables|Default|GetStartNode) (Variables|Default|GetEndNode) (.z (Variables|/Script/Engine.SceneComponent|GetRelativeLocation (Variables|Default|GetStartNodeStartPosition))) (.z (Variables|/Script/Engine.SceneComponent|GetRelativeLocation (Variables|Default|GetStartNodeEndPosition)))))

(event Collision|EventActorBeginOverlap
  (params (OtherActor :type Actor%20Object%20Reference)))

(event EventTick
  (params (DeltaSeconds :type Float%20%28single-precision%29))
  (CallFunction|LaserTrace))

(fn ConstructionScript)

(fn LaserTrace
  (bind _outhit (Collision|LineTraceByChannel (Transformation|GetWorldLocation (Variables|Default|GetStartNode)) (Transformation|GetWorldLocation (Variables|Default|GetEndNode)) "TraceTypeQuery2" false 0 "ForDuration" true "(R=1.000000,G=0.000000,B=0.143238,A=1.000000)" "(R=0.000000,G=1.000000,B=0.000000,A=1.000000)" 0.0))
  (bind _asball_character (Utilities|Casting|CastToBallCharacter (.HitActor (Collision|BreakHitResult _outhit))))
  (Variables|/Game/Blueprints/BallCharacter.BallCharacter_C|SetHealth _asball_character (Math|Float|Clamp(Float) (- (Variables|/Game/Blueprints/BallCharacter.BallCharacter_C|GetHealth _asball_character) 0.3) 0.0 1e+02))
  (bind _asbp_player_controller (Utilities|Casting|CastToBP_PlayerController (Game|GetPlayerController 0)))
  (Default|UpdateHealth _asbp_player_controller (Math|Float|Clamp(Float) (- (Variables|/Game/Blueprints/BallCharacter.BallCharacter_C|GetHealth _asball_character) 0.3) 0.0 1e+02))
  (if (<= (Math|Float|Clamp(Float) (- (Variables|/Game/Blueprints/BallCharacter.BallCharacter_C|GetHealth _asball_character) 0.3) 0.0 1e+02) 0.0)
    (Variables|/Game/Blueprints/BP_PlayerController.BP_PlayerController_C|SetIsGameLost _asbp_player_controller true)))